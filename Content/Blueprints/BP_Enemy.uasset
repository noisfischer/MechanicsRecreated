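; BP_Enemy is an enemy protected by a shield that flashlight damage drains, exposing it to melee.
; Each flashlight hit lowers the clamped shield value and notifies the shield widget.
; At zero, a DoOnce plays a sped-up reaction montage, removes the widget, adds a "shielddown" tag and sets ShieldDown.
; Melee damage only takes effect once the shield is down, switching the mesh to ragdoll physics.
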(event EventMeleeDamage
  (params (damage :type Float%20%28double-precision%29))
  (if (Variables|Default|GetshieldDown)
    (Physics|SetSimulatePhysics (Variables|Character|GetMesh) true)))

(event EventFlashlightDamage
  (params (damage :type Float%20%28double-precision%29))
  (Variables|Default|SetcurrentShield (Math|Float|Clamp(Float) (- (Variables|Default|GetcurrentShield) damage) 0.0 (Variables|Default|GetmaxShield)))
  (if (== (Variables|Default|GetcurrentShield) 0.0)
    (Utilities|FlowControl|DoOnce false
      (:Completed
        (Animation|Montage|PlayMontage (Variables|Character|GetMesh) "/Game/David/Animations/David_Reaction_Montage.David_Reaction_Montage" 2.0
          (:then
            (Components|DestroyComponent (Variables|Default|GetEnemyShieldWidget))
            (Utilities|Array|Add (Variables|Actor|GetTags) "shielddown")
            (Variables|Default|SetshieldDown true)))))
    (else
      (Class|BPIDamage|FlashlightDamage(Message) (UserInterface|GetWidget (Variables|Default|GetEnemyShieldWidget)) (Variables|Default|GetcurrentShield)))))

(fn ConstructionScript)