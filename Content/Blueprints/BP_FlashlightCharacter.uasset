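; Player character with a flashlight and follow camera that aims and zooms while the left mouse button is held.
; Press plays the Zoom timeline and starts the Aim montage at zero play rate as a held pose; release stops it and reverses Zoom.
; Timeline updates lerp camera FOV, boom Y offset, and spotlight intensity and cone angles, narrowing view and beam while brightening the light.
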(event Input|MouseEvents|LeftMouseButton
  (params (Key :type Key%20Structure :default "None"))
  (:Pressed
    (Audio|Components|Audio|Play (Variables|Default|GetZoom))
    (Animation|Montage|PlayMontage (Variables|Character|GetMesh) "/Game/David/Animations/Aim.Aim" 0.0))
  (:Released
    (Animation|StopAnimMontage "/Game/David/Animations/Aim.Aim")
    (Utilities|String|Reverse (Variables|Default|GetZoom))))

(fn ConstructionScript)