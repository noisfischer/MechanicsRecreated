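; Flashlight component that turns the player character's spotlight into a weapon against shielded enemies.
; On BeginPlay it caches the BP_ThirdPersonCharacter, then each Tick line-traces on the Camera channel from the spotlight along its forward vector up to FlashRange.
; Hit actors tagged "enemy" but not "shielddown" receive FlashlightDamageMessage with Damage every frame, and a small spark emitter spawns at the hit point.
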(event EventBeginPlay
  (bind _asbp_third_person_character (Utilities|Casting|CastToBP_ThirdPersonCharacter (Game|GetPlayerCharacter 0)))
  (Variables|Default|SetPlayerRef _asbp_third_person_character))

(event EventTick
  (params (DeltaSeconds :type Float%20%28single-precision%29))
  (bind _playerref (Variables|Default|GetPlayerRef))
  (bind _spotlight (Variables|/Game/Blueprints/BP_ThirdPersonCharacter.BP_ThirdPersonCharacter_C|GetSpotLight _playerref))
  (bind _returnvalue (Transformation|GetWorldLocation _spotlight))
  (bind (_outhit _returnvalue_2) (Collision|LineTraceByChannel _returnvalue (+ _returnvalue (* (Math|Vector|GetForwardVector _spotlight) (Variables|Default|GetFlashRange))) "TraceTypeQuery2" false 0 "None" true "(R=1.000000,G=0.000000,B=0.000000,A=1.000000)" "(R=0.000000,G=1.000000,B=0.000000,A=1.000000)" 0.1))
  (if _returnvalue_2
    (Utilities|IsValid (.HitActor (Collision|BreakHitResult _outhit))
      (:Is%20Valid
        (Variables|Default|SetHitLocation (.Location (Collision|BreakHitResult _outhit)))
        (Variables|Default|SetHit%20Actor (.HitActor (Collision|BreakHitResult _outhit)))
        (if (and (Actor|ActorHasTag (.HitActor (Collision|BreakHitResult _outhit)) "enemy") (not (Actor|ActorHasTag (.HitActor (Collision|BreakHitResult _outhit)) "shielddown")))
          (Class|BPIDamage|FlashlightDamage(Message) (Variables|Default|GetHit%20Actor) (Variables|Default|GetDamage))
          (Effects|SpawnEmitteratLocation "/Game/Realistic_Starter_VFX_Pack_Vol2/Particles/Sparks/P_Sparks_A.P_Sparks_A" (Variables|Default|GetHitLocation) "0, 0, 0" "0.100000,0.100000,0.100000"))))))